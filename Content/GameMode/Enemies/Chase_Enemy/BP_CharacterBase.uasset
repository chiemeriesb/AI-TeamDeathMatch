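; Base character Blueprint for the Chase_Enemy game mode, handling health, death, team tag, ammo and score.
; Damage clamps health, and death stops the AI brain logic before calling CallDeath; ScoreSystem increments Score for dead opposing-team characters.
; BeginPlay adds a Score widget, and a Delay-gated Tick runs a countdown that quits the game at zero.
; Shoot only line-traces without using the hit, CanAttack/CanShoot always return true, and bullet-spawn logic is disconnected.
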(event `self.ReceiveBeginPlay`
  (bind _returnvalue (`|CreateWidget` "/Game/GameMode/ScoreBoard/Score.Score_C"))
  (`UserWidget.AddToViewport` _returnvalue 0))

(event `self.ReceiveAnyDamage`
  (params (Damage :type "Float (single-precision)") (DamageType :type "DamageType Object Reference") (InstigatedBy :type "Controller Object Reference") (DamageCauser :type "Actor Object Reference"))
  (if (not (`self.IsDead?`))
    (bind _output_get (set `self.CurrentHealth` (`KismetMathLibrary.FClamp` (- (`self.CurrentHealth`) Damage) 0.0 (`self.MaxHealth`))))
    (if (<= _output_get 0.0)
      (set `self.IsDead?` true)
      (`BrainComponent.StopLogic` (`AIController.BrainComponent` (`AIBlueprintHelperLibrary.GetAIController` self)) "Dead")
      (`self.Death` self))))

(event `/Game/GameMode/Enemies/I_Shooter.Shoot`
  (`/Engine/EditorBlueprintResources/StandardMacros.IsValid` (`AIController.GetFocusActor` (`AIBlueprintHelperLibrary.GetAIController` self))
    (:`Is Valid`
      (`KismetSystemLibrary.LineTraceSingle` (0.0 0.0 0.0) (0.0 0.0 0.0) "TraceTypeQuery1"))))

(event `self.ReceiveTick`
  (params (DeltaSeconds :type "Float (single-precision)"))
  (`KismetSystemLibrary.Delay` 1.0)
  (if (== (`self.Seconds`) 0)
    (if (== (`self.Minutes`) 0)
      (`KismetSystemLibrary.PrintString` "Game Over")
      (`KismetSystemLibrary.QuitGame` null "Quit")
      (else
        (set `self.Seconds` 59)
        (set `self.Minutes` (- (`self.Minutes`) 1))))
    (else
      (set `self.Seconds` (- (`self.Seconds`) 1)))))

(event `ScoreSystem`
  (params (Actor :type "/Game/GameMode/Enemies/Chase_Enemy/BP_CharacterBase Object Reference"))
  (bind _asbp_character_base (cast `/Game/GameMode/Enemies/Chase_Enemy/BP_CharacterBase` Actor))
  (if (and (<= (`/Game/GameMode/Enemies/Chase_Enemy/BP_CharacterBase.CurrentHealth` _asbp_character_base) 0.0) (!= (`/Game/GameMode/Enemies/Chase_Enemy/BP_CharacterBase.TeamTag` _asbp_character_base) (`self.TeamTag`)))
    (set `self.Score` (+ (`self.Score`) 1))))

(fn `CanAttack`
  (returns (CanAttack :type Boolean))
  (return true))

(fn `CanShoot`
  (returns (Success :type Boolean))
  (return true))

(fn `Reload`
  (locals (TempAmmo :type Integer :default 0))
  (bind _maxammo (`self.MaxAmmo`))
  (set `local.TempAmmo` _maxammo)
  (set `self.MaxAmmo` (`KismetMathLibrary.Clamp` (- _maxammo (- 30 (`self.CurrentAmmo`))) 0 (`self.MaxAmmo`)))
  (set `self.CurrentAmmo` (+ (- (`local.TempAmmo`) (`self.MaxAmmo`)) (`self.CurrentAmmo`))))

(fn `Use Ammo`
  (set `self.CurrentAmmo` (`KismetMathLibrary.Clamp` (- (`self.CurrentAmmo`) 1) 0 30)))

(fn `UserConstructionScript`
  (`BlueprintGameplayTagLibrary.AddGameplayTag` (`self.ActorTagContainer`) (`self.TeamTag`)))